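; Weapon holder that follows the character's ALS looking rotation, animating first-person weapon and camera motion and exposing hand/elbow IK transforms.
; SetWeapon positions hands, pivot and camera from mesh sockets and weapon data, reapplied via a delayed Tick.
; Timelines drive aim, sprint tilt and recoil with falloff, counter-moving the weapon-attached camera during kick.
; WeaponShake, with no wired start, combines bob, sway and those rotation offsets, counter-rotating the local camera.
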(event `Recoil`
  (params (Pitch :type "Float (double-precision)") (Yaw :type "Float (double-precision)"))
  (bind _weapon (`self.Weapon`))
  (bind _wcs (`self.WCS`))
  (bind _camera (`/Game/WeaponSystem/Blueprints/AC_WCS.GetCamera` _wcs))
  ;[1 1 1] Camera and Weapon Recoil
  (set `self.Weapon Firing` true)
  (set `self.Temp Pitch` (`KismetMathLibrary.ClampAngle` (+ Pitch (`self.Temp Pitch`)) 0.0 20.0))
  (set `self.Temp Yaw` (+ Yaw (`self.Temp Yaw`)))
  (bind (_direction _alpha) (`Timeline|Recoil Animation` :!via `PlayFromStart`)
    (:`Update`
      (`/Engine/EditorBlueprintResources/StandardMacros.IsValid` (`/Game/WeaponSystem/Blueprints/AC_WCS.Current Weapon` _wcs)
        (:`Is Valid`
          (bind _returnvalue (`KismetMathLibrary.VLerp` (0.0 0.0 0.0) (`self.Weapon Recoil`) _alpha))
          (`SceneComponent.K2_SetRelativeLocation` _weapon (`self.Relative Location Interp` _weapon (+ (`self.Weapon Location`) _returnvalue)) false false)
          (`SceneComponent.K2_SetRelativeLocation` _camera (`self.Relative Location Interp` _camera (- (+ (`self.Camera Offset`) (`KismetMathLibrary.SelectVector` (0.0 0.0 0.0) (`self.Camera Hip`) (`/Game/WeaponSystem/Blueprints/AC_WCS.Aiming` _wcs))) _returnvalue)) false false) ; Fake camera opposite movement as its attached to weapon
          (bind (_direction_2 _alpha_2) (`Timeline|Recoil Removal` :!via `PlayFromStart`)
            (:`Update`
              (set `self.Temp Pitch` (`KismetMathLibrary.FClamp` (`KismetMathLibrary.Lerp` (`self.Temp Pitch`) 0.0 _alpha_2) 0.0 30.0))
              (set `self.Temp Yaw` (`KismetMathLibrary.FClamp` (`KismetMathLibrary.Lerp` (`self.Temp Yaw`) 0.0 _alpha_2) -30.0 30.0)))))))
    (:`Finished`
      (set `self.Weapon Firing` false))))

(event `Aim`
  (params (`Aim In` :type Boolean))
  (bind _wcs (`self.WCS`))
  (bind _camera_offset (`self.Camera Offset`))
  (bind _relativelocation_x (`KismetMathLibrary.BreakVector` (`SceneComponent.RelativeLocation` (`self.Handle`))))
  ;[1 1 1] Weapon movement during Aim
  (if `Aim In`
    (bind (_direction _alpha _xcurve) (`Timeline|Smooth Aim` :!label _label)
      (:`Update`
        (set `self.Weapon Location` (+ (`KismetMathLibrary.VLerp` (+ (`self.Weapon Hip`) (`KismetMathLibrary.MakeVector` (* _relativelocation_x 0.1))) (0.0 0.0 0.0) _alpha) _xcurve))
        (if (`/Game/WeaponSystem/Blueprints/AC_WCS.IsLocal` _wcs)
          (`SceneComponent.K2_SetRelativeLocation` (`/Game/WeaponSystem/Blueprints/AC_WCS.GetCamera` _wcs) (`KismetMathLibrary.VLerp` (+ _camera_offset (`self.Camera Hip`)) _camera_offset _alpha) false false))))
    (else
      (goto _label :!via `Reverse`))))

(event `self.ReceiveBeginPlay`
  (`self.Aim` false))

(event `self.ReceiveTick`
  (params (DeltaSeconds :type "Float (single-precision)"))
  (`SceneComponent.K2_SetWorldRotation` (`self.Root`) (`/Game/ALS/Blueprints/AC_ALS.LookingRotation` (`self.GetComponentByClass` (`/Game/WeaponSystem/Blueprints/AC_WCS.Character` (`self.WCS`)) "/Game/ALS/Blueprints/AC_ALS.AC_ALS_C")) false false)
  (`KismetSystemLibrary.Delay` 1.0)
  (bind _current_weapon (`/Game/WeaponSystem/Blueprints/AC_WCS.Current Weapon` (`self.WCS`))
    (:`then`
      (`self.Set Weapon` _current_weapon))
    (:`else`)))

(event `Set Weapon Multicast`
  (params (Actor :type "/Game/WeaponSystem/Blueprints/BP_Weapon Object Reference"))
  (`self.Set Weapon` Actor))

(event `Sprint`
  (params (True :type Boolean))
  (if True
    (bind (_direction _alpha) (`Timeline|Timeline_4` :!label _label_2)
      (:`Update`
        (set `self.Sprint Rotation` (* _alpha -50.0))))
    (else
      (goto _label_2 :!via `Reverse`))))

(fn `GetIKLocations`
  (returns (LeftHand :type "Transform Structure") (RightHand :type "Transform Structure") (Recoil :type "Float (double-precision)"))
  (bind (_returnvalue_location _returnvalue_rotation) (`KismetMathLibrary.BreakTransform` (`SceneComponent.K2_GetComponentToWorld` (`self.RightHand`))))
  (bind (_returnvalue_location_2 _returnvalue_rotation_2) (`KismetMathLibrary.BreakTransform` (`SceneComponent.K2_GetComponentToWorld` (`self.LeftHand`))))
  (bind _relativelocation_x (`KismetMathLibrary.BreakVector` (`SceneComponent.RelativeLocation` (`self.Weapon`))))
  (return (`KismetMathLibrary.MakeTransform` _returnvalue_location_2 _returnvalue_rotation_2 (`SceneComponent.K2_GetComponentLocation` (`self.LElbow`))) (`KismetMathLibrary.MakeTransform` _returnvalue_location _returnvalue_rotation (`SceneComponent.K2_GetComponentLocation` (`self.RightElbow`))) _relativelocation_x))

(fn `Relative Location Interp`
  (params (Component :type "SceneComponent Object Reference") (Target :type "Vector Structure") (InterpSpeed :type "Float (double-precision)" :default 20.0))
  (returns (ReturnValue :type "Vector Structure"))
  (return (`KismetMathLibrary.VInterpTo` (`SceneComponent.RelativeLocation` Component) Target (`GameplayStatics.GetWorldDeltaSeconds`) InterpSpeed)))

(fn `Relative Rotation Interp`
  (params (Component :type "SceneComponent Object Reference") (Target :type "Rotator Structure") (InterpSpeed :type "Float (double-precision)" :default 20.0))
  (returns (ReturnValue :type "Rotator Structure"))
  (return (`KismetMathLibrary.RInterpTo` (`SceneComponent.RelativeRotation` Component) Target (`GameplayStatics.GetWorldDeltaSeconds`) InterpSpeed)))

(fn `Set Weapon`
  (params (Actor :type "/Game/WeaponSystem/Blueprints/BP_Weapon Object Reference"))
  (bind _body (`/Game/WeaponSystem/Blueprints/BP_Weapon.Body` Actor))
  (bind (_returnvalue_location _returnvalue_rotation) (`KismetMathLibrary.BreakTransform` (`SceneComponent.GetSocketTransform` _body "LeftHand" "RTS_Component")))
  (bind ((`KickBack_183_A624F9774635D26D8867EFB8C7A1A641` _kickback) (`RecoilFalloffCurve_147_74B5948E45091315362FC493A8F4A62F` _recoilfalloffcurve) (`CameraOffset_179_BED30EA34D312CEE4A762C81F4DA3D1C` _cameraoffset)) (break `/Game/WeaponSystem/Blueprints/ST_WeraponAttributes` (`/Game/WeaponSystem/Blueprints/AC_WCS.WeaponData` (`self.WCS`))))
  (for _array_element (`|MakeArray` "RightHand" "LeftHand" "Pivot" :!type "Name")
    (if (not (`SceneComponent.DoesSocketExist` _body _array_element))
      (`KismetSystemLibrary.PrintText` (`|FormatText` "'{a}' Socket is missing on the weapon mesh/skeleton. This might break the Weapon Component " _array_element) true true (struct :`R` 0.890625 :`G` 0.385938 :`A` 1.0))))
  (`SceneComponent.K2_SetRelativeTransform` (`self.Scene`) (`SceneComponent.GetSocketTransform` _body "RightHand" "RTS_Component") false false)
  (`SceneComponent.K2_SetRelativeTransform` (`self.LeftHand`) (`KismetMathLibrary.MakeTransform` (+ _returnvalue_location (-5.0 -12.5 -5.0)) (`KismetMathLibrary.ComposeRotators` (struct) _returnvalue_rotation) (1.0 1.0 1.0)) false false)
  (`SceneComponent.K2_SetRelativeLocation` (`self.Handle`) (`KismetMathLibrary.MakeVector` (* -1 (.x (.location (`SceneComponent.GetSocketTransform` _body "Pivot" "RTS_Component"))))) false false)
  (set `self.Camera Offset` _cameraoffset)
  (set `self.Weapon Recoil` (`KismetMathLibrary.MakeVector` _kickback))
  (`TimelineComponent.SetFloatCurve` (`self.Recoil Removal`) _recoilfalloffcurve "Alpha")
  (`SceneComponent.K2_SetRelativeLocation` (`self.Camera`) _cameraoffset false false))

(fn `UserConstructionScript`)