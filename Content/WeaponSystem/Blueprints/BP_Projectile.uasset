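; Configurable projectile actor for the weapon system that flies via a ProjectileMovement component and destroys itself when movement stops.
; The construction script applies bullet speed and mesh from its variables.
; A single FX asset slot accepts either a Niagara or Cascade system, feeding the matching component and destroying the other.
; Mesh hits only print a debug string, with no damage logic.
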(event `self.ProjectileMovement.OnProjectileStop`
  (params (ImpactResult :type "HitResult Structure (by ref)"))
  (`self.K2_DestroyActor`))

(event `self.Mesh.OnComponentHit`
  (params (HitComponent :type "PrimitiveComponent Object Reference") (OtherActor :type "Actor Object Reference") (OtherComp :type "PrimitiveComponent Object Reference") (NormalImpulse :type "Vector Structure") (Hit :type "HitResult Structure (by ref)"))
  (`KismetSystemLibrary.PrintString` "Hello"))

(fn `UserConstructionScript`
  (bind _particle (`self.Particle`))
  (bind _niagara (`self.Niagara`))
  (set `ProjectileMovementComponent.InitialSpeed` (`self.Bullet Speed`) (`self.ProjectileMovement`))
  (`StaticMeshComponent.SetStaticMesh` (`self.Mesh`) (`self.Bullet Mesh`))
  ;[0.4193 1 0.2417] Use Niagra or Particle system based on provided asset
  (bind _fx_asset (`self.FX Asset`)
    (:`then`
      (bind _asniagara_system (cast `NiagaraSystem` _fx_asset)
        (:`then`
          (`NiagaraComponent.SetAsset` _niagara _asniagara_system)
          (`ActorComponent.K2_DestroyComponent` _particle))
        (:`CastFailed`
          (bind _asparticle_system (cast `ParticleSystem` _fx_asset))
          (`ParticleSystemComponent.SetTemplate` _particle _asparticle_system)
          (`ActorComponent.K2_DestroyComponent` _niagara))))
    (:`else`)))