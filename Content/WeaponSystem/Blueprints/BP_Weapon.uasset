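; BP_Weapon is a data-driven weapon Blueprint that configures itself from a data table row.
; Its construction script looks up the row named by the ID handle and stores it as WeaponAttributes.
; When the row is found, it applies the skeletal mesh and offset to Body, positions CameraHolder, selects the first fire mode and fills the clip ammo to clip size.
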(fn `UserConstructionScript`
  (bind (_id_datatable _id_rowname) (break `DataTableRowHandle` (`self.ID`)))
  (bind _body (`self.Body`))
  (bind _returnvalue (`|GetDataTableRow` _id_datatable _id_rowname)
    (:`then`
      (bind _output_get (set `self.Weapon Attributes` _returnvalue))
      (bind ((`Mesh_56_9313E4834B4F91EB32EB6FA9D8635CA9` _mesh) (`MeshOffset_26_A51F415E48224F3080A283AD15C26368` _meshoffset) (`CharacterWeaponBaseAnimation_197_BE03496044134477938989B64F321CDB` _characterweaponbaseanimation) (`FireModes_84_0B2FBF5E4419103968A42CA290492B5A` _firemodes) (`ClipSize_93_6B3D5348405C6791E732AA928D8EC5C9` _clipsize) (`CameraOffset_179_BED30EA34D312CEE4A762C81F4DA3D1C` _cameraoffset)) (break `/Game/WeaponSystem/Blueprints/ST_WeraponAttributes` _output_get))
      (`SkinnedMeshComponent.SetSkinnedAssetAndUpdate` _body _mesh true)
      (`SceneComponent.K2_SetRelativeTransform` _body _meshoffset false false)
      (set `self.Fire Mode` (`|GetArrayItem` _firemodes))
      (`SceneComponent.K2_SetRelativeLocation` (`self.CameraHolder`) _cameraoffset false false)
      (set `self.Clip Ammo` _clipsize))))