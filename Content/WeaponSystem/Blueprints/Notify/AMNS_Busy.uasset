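; Anim notify state "Weapon Busy" that sets the weapon state for the duration of its window in an animation.
; On begin it finds the AC_WCS component on the mesh owner and writes the notify's WeaponState value to it.
; On end it resets that state to the enum's first entry.
; Both print an error and return false if the component is missing.
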(fn `GetNotifyName`
  (returns (ReturnValue :type String))
  (return "Weapon Busy "))

(fn `Received_NotifyBegin`
  (params (MeshComp :type "SkeletalMeshComponent Object Reference") (Animation :type "AnimSequenceBase Object Reference") (TotalDuration :type "Float (double-precision)"))
  (returns (ReturnValue :type Boolean))
  (bind _returnvalue (`Actor.GetComponentByClass` (`ActorComponent.GetOwner` MeshComp) "/Game/WeaponSystem/Blueprints/AC_WCS.AC_WCS_C"))
  (`/Engine/EditorBlueprintResources/StandardMacros.IsValid` _returnvalue
    (:`Is Valid`
      (set `/Game/WeaponSystem/Blueprints/AC_WCS.WeaponState` (`self.Weapon State`) _returnvalue)
      (return true))
    (:`Is Not Valid`
      (`KismetSystemLibrary.PrintString` null "Weapon Component Doesnt exist on Player")
      (return false))))

(fn `Received_NotifyEnd`
  (params (MeshComp :type "SkeletalMeshComponent Object Reference") (Animation :type "AnimSequenceBase Object Reference"))
  (returns (ReturnValue :type Boolean))
  (bind _returnvalue (`Actor.GetComponentByClass` (`ActorComponent.GetOwner` MeshComp) "/Game/WeaponSystem/Blueprints/AC_WCS.AC_WCS_C"))
  (`/Engine/EditorBlueprintResources/StandardMacros.IsValid` _returnvalue
    (:`Is Valid`
      (set `/Game/WeaponSystem/Blueprints/AC_WCS.WeaponState` "NewEnumerator0" _returnvalue)
      (return true))
    (:`Is Not Valid`
      (`KismetSystemLibrary.PrintString` null "Weapon Component Doesnt exist on Player")
      (return false))))